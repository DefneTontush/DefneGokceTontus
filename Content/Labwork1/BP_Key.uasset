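; BP_Key is a key pickup for a maze game that the player collects by interacting with it.
; It caches BP_MazeGamemode on BeginPlay, and Interact overwrites the game mode's Keys value with this key's KeyNumber rather than accumulating it.
; Interact then prints an acquired message using the matching entry in Names and destroys the actor.
; The construction script applies the Material variable to the Key component.
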(event EventBeginPlay
  (bind _asbp_maze_gamemode (Utilities|Casting|CastToBP_MazeGamemode (Game|GetGameMode)))
  (Variables|Default|SetAs%20BP%20Maze%20Gamemode _asbp_maze_gamemode))

(event EventInteract
  (bind _output_get (Variables|/Game/Labwork1/BP_MazeGamemode.BP_MazeGamemode_C|SetKeys (Variables|Default|GetAs%20BP%20Maze%20Gamemode) (Variables|Default|GetKeyNumber)))
  (Development|PrintString (Utilities|String|Append "Key" (Utilities|Array|Get(acopy) (Variables|Default|GetNames) _output_get) "Acquired"))
  (Actor|DestroyActor))

(fn ConstructionScript
  (Rendering|Material|SetMaterial (Variables|Default|GetKey) 0 (Variables|Default|GetMaterial)))