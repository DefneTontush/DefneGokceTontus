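; BP_SlidingDoor is a maze door that slides open on interaction when the player holds the matching key.
; On BeginPlay it caches BP_MazeGamemode, and Interact requires that game mode's Keys value to exactly equal the door's KeyNumber.
; A match plays the DoorSlide timeline to lerp the Door between start and finish locations, otherwise it prints a wrong-key message.
; The construction script applies a configurable material to the Door.
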(event EventBeginPlay
  (bind _asbp_maze_gamemode (Utilities|Casting|CastToBP_MazeGamemode (Game|GetGameMode)))
  (Variables|Default|SetAs%20BP%20Maze%20Gamemode _asbp_maze_gamemode))

(event EventInteract
  (if (== (Variables|/Game/Labwork1/BP_MazeGamemode.BP_MazeGamemode_C|GetKeys (Variables|Default|GetAs%20BP%20Maze%20Gamemode)) (Variables|Default|GetKeyNumber))
    (bind _newtrack_0 (Timeline|DoorSlide Play)
      (:Update
        (Transformation|SetRelativeLocation (Variables|Default|GetDoor) (Math|Vector|Lerp(Vector) (Variables|Default|GetStartLocation) (Variables|Default|GetFinishLocation) _newtrack_0) false false)))
    (else
      (Development|PrintString "You do not have the correct key"))))

(fn ConstructionScript
  (Rendering|Material|SetMaterial (Variables|Default|GetDoor) 0 (Variables|Default|GetMaterial)))