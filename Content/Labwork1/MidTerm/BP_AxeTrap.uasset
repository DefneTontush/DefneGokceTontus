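; BP_AxeTrap is a swinging axe trap that damages the third-person character.
; Overlapping any of four rope triggers plays the Axe timeline, which lerps the Sphere component's relative rotation between start and end rotations.
; Character overlap with Cube subtracts Damage directly from the character's Health variable, while Cube1's overlap only casts and has no further effect.
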(event OnComponentBeginOverlap(Rope)
  (params (OverlappedComponent :type Primitive%20Component%20Object%20Reference) (OtherActor :type Actor%20Object%20Reference) (OtherComp :type Primitive%20Component%20Object%20Reference) (OtherBodyIndex :type Integer) (bFromSweep :type Boolean) (SweepResult :type Hit%20Result%20Structure%20%28by%20ref%29))
  (Utilities|Casting|CastToBP_ThirdPersonCharacter OtherActor)
  (bind _newtrack_0 (Timeline|Axe Play)
    (:Update
      (Transformation|SetRelativeRotation (Variables|Default|GetSphere) (Math|Rotator|Lerp(Rotator) (Variables|Default|GetStartRotation) (Variables|Default|GetEndRotation) _newtrack_0) false false))))

(event OnComponentBeginOverlap(Rope1)
  (params (OverlappedComponent :type Primitive%20Component%20Object%20Reference) (OtherActor :type Actor%20Object%20Reference) (OtherComp :type Primitive%20Component%20Object%20Reference) (OtherBodyIndex :type Integer) (bFromSweep :type Boolean) (SweepResult :type Hit%20Result%20Structure%20%28by%20ref%29))
  (Utilities|Casting|CastToBP_ThirdPersonCharacter OtherActor)
  (bind _newtrack_0 (Timeline|Axe Play)
    (:Update
      (Transformation|SetRelativeRotation (Variables|Default|GetSphere) (Math|Rotator|Lerp(Rotator) (Variables|Default|GetStartRotation) (Variables|Default|GetEndRotation) _newtrack_0) false false))))

(event OnComponentBeginOverlap(Rope2)
  (params (OverlappedComponent :type Primitive%20Component%20Object%20Reference) (OtherActor :type Actor%20Object%20Reference) (OtherComp :type Primitive%20Component%20Object%20Reference) (OtherBodyIndex :type Integer) (bFromSweep :type Boolean) (SweepResult :type Hit%20Result%20Structure%20%28by%20ref%29))
  (Utilities|Casting|CastToBP_ThirdPersonCharacter OtherActor)
  (bind _newtrack_0 (Timeline|Axe Play)
    (:Update
      (Transformation|SetRelativeRotation (Variables|Default|GetSphere) (Math|Rotator|Lerp(Rotator) (Variables|Default|GetStartRotation) (Variables|Default|GetEndRotation) _newtrack_0) false false))))

(event OnComponentBeginOverlap(Rope3)
  (params (OverlappedComponent :type Primitive%20Component%20Object%20Reference) (OtherActor :type Actor%20Object%20Reference) (OtherComp :type Primitive%20Component%20Object%20Reference) (OtherBodyIndex :type Integer) (bFromSweep :type Boolean) (SweepResult :type Hit%20Result%20Structure%20%28by%20ref%29))
  (Utilities|Casting|CastToBP_ThirdPersonCharacter OtherActor)
  (bind _newtrack_0 (Timeline|Axe Play)
    (:Update
      (Transformation|SetRelativeRotation (Variables|Default|GetSphere) (Math|Rotator|Lerp(Rotator) (Variables|Default|GetStartRotation) (Variables|Default|GetEndRotation) _newtrack_0) false false))))

(event OnComponentBeginOverlap(Cube)
  (params (OverlappedComponent :type Primitive%20Component%20Object%20Reference) (OtherActor :type Actor%20Object%20Reference) (OtherComp :type Primitive%20Component%20Object%20Reference) (OtherBodyIndex :type Integer) (bFromSweep :type Boolean) (SweepResult :type Hit%20Result%20Structure%20%28by%20ref%29))
  (bind _asbp_third_person_character (Utilities|Casting|CastToBP_ThirdPersonCharacter OtherActor))
  (Variables|/Game/ThirdPerson/Blueprints/BP_ThirdPersonCharacter.BP_ThirdPersonCharacter_C|SetHealth _asbp_third_person_character (- (Variables|/Game/ThirdPerson/Blueprints/BP_ThirdPersonCharacter.BP_ThirdPersonCharacter_C|GetHealth _asbp_third_person_character) (Variables|Default|GetDamage))))

(event OnComponentBeginOverlap(Cube1)
  (params (OverlappedComponent :type Primitive%20Component%20Object%20Reference) (OtherActor :type Actor%20Object%20Reference) (OtherComp :type Primitive%20Component%20Object%20Reference) (OtherBodyIndex :type Integer) (bFromSweep :type Boolean) (SweepResult :type Hit%20Result%20Structure%20%28by%20ref%29))
  (Utilities|Casting|CastToBP_ThirdPersonCharacter OtherActor))

(fn ConstructionScript)