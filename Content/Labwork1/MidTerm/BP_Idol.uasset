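; BP_Idol is an interactable idol that disables one type of trap in the level when used.
; On Interact, IdolIndex selects the stake, poison or axe trap class, destroys the actor returned by GetActorOfClass for it, then destroys the idol itself.
; The construction script applies the Material variable to the Idol mesh, so each placed idol can look different.
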(event EventInteract
  (switch int (Variables|Default|GetIdolIndex)
    (:0
      (bind _returnvalue (Actor|GetActorOfClass "/Game/Labwork1/MidTerm/BP_StakeTrap.BP_StakeTrap_C"))
      (Actor|DestroyActor _returnvalue))
    (:1
      (bind _returnvalue_2 (Actor|GetActorOfClass "/Game/Labwork1/MidTerm/BP_PoisonTrap.BP_PoisonTrap_C"))
      (Actor|DestroyActor _returnvalue_2))
    (:2
      (bind _returnvalue_3 (Actor|GetActorOfClass "/Game/Labwork1/MidTerm/BP_AxeTrap.BP_AxeTrap_C"))
      (Actor|DestroyActor _returnvalue_3)))
  (Actor|DestroyActor))

(fn ConstructionScript
  (Rendering|Material|SetMaterial (Variables|Default|GetIdol) 0 (Variables|Default|GetMaterial)))